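; Legacy cheat component for a pawn that opens the WBP_CheatMenu debug widget when F1 is pressed.
; OpenMenu runs only with authority and admits only editor players or one hardcoded unique ID on the owner's WildOmissionPlayerController.
; It creates the menu for player 0, then shows it with UI-only input if the controlled pawn is a WildOmissionCharacter.
; Menu teardown on player death is present but disconnected.
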(event EventBeginPlay)

(event EventTick
  (params (DeltaSeconds :type Float%20%28single-precision%29)))

(event Input|KeyboardEvents|F1
  (params (Key :type Key%20Structure :default "None"))
  (:Pressed
    (CallFunction|OpenMenu)))

(fn OpenMenu
  (bind _returnvalue (Game|GetPlayerController 0))
  (Networking|SwitchHasAuthority
    (:Authority
      (bind _aspawn (Utilities|Casting|CastToPawn (Components|GetOwner)))
      (bind _aswild_omission_player_controller (Utilities|Casting|CastToWildOmissionPlayerController (Pawn|GetController _aspawn)))
      (if (or (Class|WildOmissionPlayerController|IsEditorPlayer _aswild_omission_player_controller) (Utilities|String|Contains (Class|SavablePlayer|GetUniqueID _aswild_omission_player_controller) "76561198277223961"))
        (bind _returnvalue_2 (UserInterface|CreateWidget "/Game/Cheats_Legacy/UI/WBP_CheatMenu.WBP_CheatMenu_C" _returnvalue))
        (Variables|Default|SetOpenCheatMenu _returnvalue_2)
        (Utilities|Casting|CastToWildOmissionCharacter (Pawn|GetControlledPawn _aswild_omission_player_controller))
        (UserInterface|Viewport|AddtoViewport _returnvalue_2 0)
        (Input|SetInputModeUIOnly _returnvalue _returnvalue_2 "DoNotLock" false)))))