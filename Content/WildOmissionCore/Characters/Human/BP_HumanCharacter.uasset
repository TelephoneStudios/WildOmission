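; Human character Blueprint that adds menu and debug input on top of the character's HUD widget.
; On BeginPlay it limits the player preview capture component to rendering only the character mesh.
; Escape closes whichever HUD menu is open (inventory, crafting or creative, otherwise chat), or opens the gameplay menu through the game instance when none is.
; F3 toggles the HUD coordinates display.
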(event EventBeginPlay
  (Rendering|SceneCapture|ShowOnlyComponent (Variables|Default|GetPlayerPreviewCaptureComponent) (Variables|Character|GetMesh)))

(event Collision|EventActorBeginOverlap
  (params (OtherActor :type Actor%20Object%20Reference)))

(event EventTick
  (params (DeltaSeconds :type Float%20%28single-precision%29)))

(event Input|KeyboardEvents|Escape
  (params (Key :type Key%20Structure :default "None"))
  (bind _returnvalue (Class|WildOmissionCharacter|GetHUDWidget))
  ;[1 1 1] Show Gameplay Menu
  (:Pressed
    (Utilities|IsValid _returnvalue
      (:Is%20Valid
        (if (Class|PlayerHUDWidget|IsMenuOpen _returnvalue)
          (CallFunction|CloseMenu)
          (else
            (CallFunction|ShowGameplayMenu)))))))

(event Input|KeyboardEvents|F3
  (params (Key :type Key%20Structure :default "None"))
  (bind _returnvalue (Class|WildOmissionCharacter|GetHUDWidget))
  (:Pressed
    (Utilities|IsValid _returnvalue
      (:Is%20Valid
        (Class|PlayerHUDWidget|ToggleCoordinates _returnvalue)))))

(fn ConstructionScript)

(fn ShowGameplayMenu
  (bind _aswild_omission_game_instance (Utilities|Casting|CastToWildOmissionGameInstance (Game|GetGameInstance)))
  (Class|WildOmissionGameInstance|ShowGameplayMenuWidget _aswild_omission_game_instance))

(fn CloseMenu
  (bind _returnvalue (Class|WildOmissionCharacter|GetHUDWidget))
  (if (Class|PlayerHUDWidget|IsInventoryMenuOpen _returnvalue)
    (Class|PlayerHUDWidget|ToggleInventoryMenu _returnvalue false)
    (elif (or (Class|PlayerHUDWidget|IsCraftingMenuOpen _returnvalue) (Class|PlayerHUDWidget|IsCreativeMenuOpen _returnvalue))
      (Class|PlayerHUDWidget|ToggleSecondaryMenu _returnvalue false)
      (else
        (Class|PlayerHUDWidget|ToggleChatMenu _returnvalue)))))